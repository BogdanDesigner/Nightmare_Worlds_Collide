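; BP_Key is a key pickup that the first-person character collects by pressing E nearby.
; Overlapping its sphere shows a billboard, enables input and opens a gate; ending the overlap hides the billboard and disables input without closing the gate.
; Pressing E sets HasKey on the cached character, then a DoOnce plays the pickup sound and destroys the actor.
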(event `Key|E` :consume false
  (params (Key :type "Key Structure"))
  ;[1 1 1] Key Setup
  (:`Pressed`
    (`/Engine/EditorBlueprintResources/StandardMacros.Gate` true :!label _label
      (:`Exit`
        (set `/Game/FP_Horror_Starter_Kit/PlayerCharacterExample/Blueprints/FirstPersonCharacter.HasKey` true (stale `self.Sphere.OnComponentBeginOverlap` _asfirst_person_character))
        (`/Engine/EditorBlueprintResources/StandardMacros.DoOnce` false
          (:`Completed`
            (`GameplayStatics.PlaySoundAtLocation` "/Game/Ben/AtompshericSounds/SM_PickUp.SM_PickUp" (`self.K2_GetActorLocation`) (struct) 1.0 1.0 0.0 null null null)
            (`self.K2_DestroyActor`)))))))

(event `self.Sphere.OnComponentBeginOverlap`
  (params (OverlappedComponent :type "PrimitiveComponent Object Reference") (OtherActor :type "Actor Object Reference") (OtherComp :type "PrimitiveComponent Object Reference") (OtherBodyIndex :type Integer) (bFromSweep :type Boolean) (SweepResult :type "HitResult Structure (by ref)"))
  ;[1 1 1] Key Setup
  (bind _asfirst_person_character (cast `/Game/FP_Horror_Starter_Kit/PlayerCharacterExample/Blueprints/FirstPersonCharacter` OtherActor))
  (`self.EnableInput` (`GameplayStatics.GetPlayerController` 0))
  (`SceneComponent.SetVisibility` (`self.Billboard`) true false)
  (goto _label :!via `Open`))

(event `self.Sphere.OnComponentEndOverlap`
  (params (OverlappedComponent :type "PrimitiveComponent Object Reference") (OtherActor :type "Actor Object Reference") (OtherComp :type "PrimitiveComponent Object Reference") (OtherBodyIndex :type Integer))
  ;[1 1 1] Key Setup
  (`self.DisableInput` (`GameplayStatics.GetPlayerController` 0))
  (`SceneComponent.SetVisibility` (`self.Billboard`) false false))

(fn `UserConstructionScript`)