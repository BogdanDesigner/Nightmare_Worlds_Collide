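; BP_Door1 is an interactable swinging door that the first-person character opens and closes with E, optionally requiring a key.
; Entering its Box trigger enables input, opens a gate and shows a prompt billboard; leaving disables input and hides both billboards.
; A FlipFlop alternately plays and reverses a timeline that drives the mesh yaw.
; When NeedsKey is set and HasKey is false, a second billboard appears, then both hide after a short delay.
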(event `Key|E` :consume false
  (params (Key :type "Key Structure"))
  ;[1 1 1] Door Setup
  (:`Pressed`
    (`/Engine/EditorBlueprintResources/StandardMacros.Gate` true :!label _label
      (:`Exit`
        (bind _asfirst_person_character (cast `/Game/FP_Horror_Starter_Kit/PlayerCharacterExample/Blueprints/FirstPersonCharacter` (stale `self.Box.OnComponentBeginOverlap` OtherActor)))
        (if (`self.NeedsKey?`)
          (if (`/Game/FP_Horror_Starter_Kit/PlayerCharacterExample/Blueprints/FirstPersonCharacter.HasKey` _asfirst_person_character)
            (`/Engine/EditorBlueprintResources/StandardMacros.FlipFlop` :!label _label_2
              (:`A`
                (bind (_direction _movement) (`Timeline|Door Open/Close` :!label _label_3)
                  (:`Update`
                    (`SceneComponent.K2_SetRelativeRotation` (`self.StaticMesh`) (`KismetMathLibrary.MakeRotator` 0.0 0.0 _movement) false false))))
              (:`B`
                (goto _label_3 :!via `Reverse`)))
            (else
              (`SceneComponent.SetVisibility` (`self.Billboard`) true false)
              (`KismetSystemLibrary.Delay` 2.0)
              (`SceneComponent.SetVisibility` (`self.Billboard`) false false :!label _label_4)
              (`SceneComponent.SetVisibility` (`self.Billboard1`) false false)))
          (else
            (goto _label_2)))))))

(event `self.Box.OnComponentBeginOverlap`
  (params (OverlappedComponent :type "PrimitiveComponent Object Reference") (OtherActor :type "Actor Object Reference") (OtherComp :type "PrimitiveComponent Object Reference") (OtherBodyIndex :type Integer) (bFromSweep :type Boolean) (SweepResult :type "HitResult Structure (by ref)"))
  ;[1 1 1] Door Setup
  (`|ExecutionSequence`
    (:`then_0`
      (`self.EnableInput` (`GameplayStatics.GetPlayerController` 0))
      (goto _label :!via `Open`))
    (:`then_1`
      (`SceneComponent.SetVisibility` (`self.Billboard1`) true false))))

(event `self.Box.OnComponentEndOverlap`
  (params (OverlappedComponent :type "PrimitiveComponent Object Reference") (OtherActor :type "Actor Object Reference") (OtherComp :type "PrimitiveComponent Object Reference") (OtherBodyIndex :type Integer))
  ;[1 1 1] Door Setup
  (`self.DisableInput` (`GameplayStatics.GetPlayerController` 0))
  (goto _label_4))

(fn `UserConstructionScript`)