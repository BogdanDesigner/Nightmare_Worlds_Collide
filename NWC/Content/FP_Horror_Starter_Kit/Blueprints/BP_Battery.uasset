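; Battery pickup for the horror starter kit that tops up the first-person character's BatteryPower by a fixed amount.
; Overlapping the sphere enables input, then a successful character cast shows the billboard prompt and opens a gate for the E key.
; Pressing E adds the charge and destroys the pickup.
; Leaving the sphere disables input and hides the billboard, but never closes the gate.
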(event `Key|E` :consume false
  (params (Key :type "Key Structure"))
  ;[1 1 1] Battery Setup
  (:`Pressed`
    (`/Engine/EditorBlueprintResources/StandardMacros.Gate` true :!label _label
      (:`Exit`
        (set `/Game/FP_Horror_Starter_Kit/PlayerCharacterExample/Blueprints/FirstPersonCharacter.Battery Power` (+ (`/Game/FP_Horror_Starter_Kit/PlayerCharacterExample/Blueprints/FirstPersonCharacter.Battery Power` (stale `self.Sphere.OnComponentBeginOverlap` _asfirst_person_character)) 0.2) (stale `self.Sphere.OnComponentBeginOverlap` _asfirst_person_character))
        (`self.K2_DestroyActor`)))))

(event `self.Sphere.OnComponentBeginOverlap`
  (params (OverlappedComponent :type "PrimitiveComponent Object Reference") (OtherActor :type "Actor Object Reference") (OtherComp :type "PrimitiveComponent Object Reference") (OtherBodyIndex :type Integer) (bFromSweep :type Boolean) (SweepResult :type "HitResult Structure (by ref)"))
  ;[1 1 1] Battery Setup
  (`self.EnableInput` (`GameplayStatics.GetPlayerController` 0))
  (bind _asfirst_person_character (cast `/Game/FP_Horror_Starter_Kit/PlayerCharacterExample/Blueprints/FirstPersonCharacter` OtherActor))
  (`SceneComponent.SetVisibility` (`self.Billboard`) true false)
  (goto _label :!via `Open`))

(event `self.Sphere.OnComponentEndOverlap`
  (params (OverlappedComponent :type "PrimitiveComponent Object Reference") (OtherActor :type "Actor Object Reference") (OtherComp :type "PrimitiveComponent Object Reference") (OtherBodyIndex :type Integer))
  ;[1 1 1] Battery Setup
  (`self.DisableInput` (`GameplayStatics.GetPlayerController` 0))
  (`SceneComponent.SetVisibility` (`self.Billboard`) false false))

(fn `UserConstructionScript`)