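; BP_PuzzleWall is an interactable wall that gives the player access to the jigsaw puzzle until it is solved.
; Its box collision shows the WBP_EnterPuzzle prompt on overlap and clears all widgets when overlap ends.
; Interact calls OpenJigsawBoard on the BP_ThirdPersonCharacter player.
; Tick polls IsSolved and, once true, removes all widgets and disables the box collision every frame.
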(event `self.ReceiveTick`
  (params (DeltaSeconds :type "Float (single-precision)"))
  ;[0.9488 1 0.3383] Checking whether or not puzzle is solve?
  (if (`self.IsSolved?`)
    (`WidgetLayoutLibrary.RemoveAllWidgets`)
    (`PrimitiveComponent.SetCollisionEnabled` (`self.Box`) "NoCollision")))

(event `self.Box.OnComponentBeginOverlap`
  (params (OverlappedComponent :type "PrimitiveComponent Object Reference") (OtherActor :type "Actor Object Reference") (OtherComp :type "PrimitiveComponent Object Reference") (OtherBodyIndex :type Integer) (bFromSweep :type Boolean) (SweepResult :type "HitResult Structure (by ref)"))
  ;[1 1 0.3185] Showing Tips or Controls to player when begin overlap withe the box collision
  (if (not (`self.IsSolved?`))
    (bind _returnvalue (`|CreateWidget` "/Game/Jigsaw_Puzzle/Widgets/WBP_EnterPuzzle.WBP_EnterPuzzle_C"))
    (`UserWidget.AddToViewport` _returnvalue 0)))

(event `self.Box.OnComponentEndOverlap`
  (params (OverlappedComponent :type "PrimitiveComponent Object Reference") (OtherActor :type "Actor Object Reference") (OtherComp :type "PrimitiveComponent Object Reference") (OtherBodyIndex :type Integer))
  ;[1 1 0.3185] Removing Tips or Controls from player screen when the player is no more overlaping with the box collision
  (if (not (`self.IsSolved?`))
    (`WidgetLayoutLibrary.RemoveAllWidgets`)))

(fn `Interact`
  (params (Interactor :type "Character Object Reference"))
  (returns (`Interact?` :type Boolean))
  ;[0.9851 1 0.2895] Can open Jigsaw Puzzle only hen the player is overlap with box collision
  (if (not (`self.IsSolved?`))
    (bind _asbp_third_person_character (cast `/Game/Jigsaw_Puzzle/Core/BP_ThirdPersonCharacter` (`GameplayStatics.GetPlayerCharacter` 0)))
    (`/Game/Jigsaw_Puzzle/Core/BP_ThirdPersonCharacter.OpenJigsawBoard` _asbp_third_person_character)
    (return true)))

(fn `UserConstructionScript`)