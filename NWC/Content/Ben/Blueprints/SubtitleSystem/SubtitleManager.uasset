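; SubtitleManager shows subtitles on screen, stepping through lines stored in a data table.
; On BeginPlay it creates a BP_Subtitle widget, then clears it and binds that clear event to the FirstPersonCharacter's SubtitleClear dispatcher.
; ShowSubtitle forwards a table and first-line flag to ShowNextSubtitle, which displays the row at CurrentRow and increments it, resetting to zero for first lines.
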(event `self.ReceiveBeginPlay`
  (`|ExecutionSequence`
    (:`then_0`
      (bind _returnvalue (`|CreateWidget` "/Game/Ben/Blueprints/SubtitleSystem/BP_Subtitle.BP_Subtitle_C"))
      (bind _output_get (set `self.SubtitleWidgetREF` _returnvalue))
      (`UserWidget.AddToViewport` _output_get 0)
      (`self.SubtitlesClear`))))

(event `SubtitlesClear`
  (bind _asfirst_person_character (cast `/Game/FP_Horror_Starter_Kit/PlayerCharacterExample/Blueprints/FirstPersonCharacter` (`GameplayStatics.GetPlayerCharacter` 0)))
  (`/Game/Ben/Blueprints/SubtitleSystem/BP_Subtitle.DisplaySubtitle` (`self.SubtitleWidgetREF`) "")
  (add `/Game/FP_Horror_Starter_Kit/PlayerCharacterExample/Blueprints/FirstPersonCharacter.SubtitleClear` _asfirst_person_character (delegate `SubtitlesClear`)))

(event `ShowNextSubtitle`
  (params (FirstLine :type Boolean) (SubtitleList :type "DataTable Object Reference"))
  (set `self.CurrentSubtitleList` SubtitleList)
  (if FirstLine
    (set `self.CurrentRow` 0)
    (bind _outrownames (`DataTableFunctionLibrary.GetDataTableRowNames` (`self.CurrentSubtitleList`)))
    (bind _returnvalue (`|GetDataTableRow` (`self.CurrentSubtitleList`) (`|GetArrayItem` _outrownames (`self.CurrentRow`)))
      (:`then`
        (`/Game/Ben/Blueprints/SubtitleSystem/BP_Subtitle.DisplaySubtitle` (`self.SubtitleWidgetREF`) (`.SubtitleToShow_3_ADEE51344F354F45823B109BF4F548CC` (break `/Game/Ben/Blueprints/SubtitleSystem/SubtitleStruct` _returnvalue)))
        (`/Engine/EditorBlueprintResources/StandardMacros.IncrementInt` (`self.CurrentRow`))))
    (else
      (bind _outrownames_2 (`DataTableFunctionLibrary.GetDataTableRowNames` (`self.CurrentSubtitleList`)))
      (bind _returnvalue_2 (`|GetDataTableRow` (`self.CurrentSubtitleList`) (`|GetArrayItem` _outrownames_2 (`self.CurrentRow`)))
        (:`then`
          (`/Game/Ben/Blueprints/SubtitleSystem/BP_Subtitle.DisplaySubtitle` (`self.SubtitleWidgetREF`) (`.SubtitleToShow_3_ADEE51344F354F45823B109BF4F548CC` (break `/Game/Ben/Blueprints/SubtitleSystem/SubtitleStruct` _returnvalue_2)))
          (`/Engine/EditorBlueprintResources/StandardMacros.IncrementInt` (`self.CurrentRow`)))))))

(fn `ShowSubtitle`
  (params (`First Line` :type Boolean) (SubtitleList :type "DataTable Object Reference"))
  (`self.ShowNextSubtitle` `First Line` SubtitleList))

(fn `UserConstructionScript`)