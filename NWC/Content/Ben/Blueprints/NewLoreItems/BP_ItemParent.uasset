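; Parent Blueprint for lore items the player can pick up, inspect and drop, with an overlap box toggling a billboard prompt.
; Interacting attaches the item to the player's hold component, or starts inspection if something is already held.
; Inspection shows a description widget and moves input from player to item for drag rotation and wheel zoom along the camera's view.
; Interaction input ends inspection; DropItem detaches the item and restores physics.
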(event `/Game/Ben/Blueprints/NewLoreItems/BP_Interact_Interface.LookAt`
  (params (PlayerCharacter :type "/Game/QuestKitMini1/Demo/FirstPersonBP/FirstPersonCharacter Object Reference")))

(event `InputAction|Interaction`
  (params (Key :type "Key Structure"))
  (:`Pressed`
    (`self.Stop Inspect`)))

(event `Key|LeftMouseButton`
  (params (Key :type "Key Structure"))
  ;[1 0.7242 0.3207] Inspect Rotation
  (:`Pressed`
    (set `self.Rotating` true))
  (:`Released`
    (set `self.Rotating` false)))

(event `/Game/Ben/Blueprints/NewLoreItems/BP_Interact_Interface.InteractWith`
  (params (PlayerCharacter :type "/Game/FP_Horror_Starter_Kit/PlayerCharacterExample/Blueprints/FirstPersonCharacter Object Reference"))
  ;[1 1 1] Interact
  (bind _output_get (set `self.Player Character` PlayerCharacter))
  (`/Game/FP_Horror_Starter_Kit/PlayerCharacterExample/Blueprints/FirstPersonCharacter.CurrentHeld` _output_get
    (:`then`
      (`self.StartInspect`))
    (:`else`
      (`self.Pick Up`))))

(event `InputAxisKey|MouseX`
  (params (AxisValue :type "Float (single-precision)"))
  ;[1 0.7242 0.3207] Inspect Rotation
  (if (`self.Rotating`)
    (`self.K2_SetActorRotation` (`KismetMathLibrary.ComposeRotators` (`self.K2_GetActorRotation`) (`KismetMathLibrary.MakeRotator` 0.0 0.0 (* AxisValue -5.0))))))

(event `self.Box.OnComponentBeginOverlap`
  (params (OverlappedComponent :type "PrimitiveComponent Object Reference") (OtherActor :type "Actor Object Reference") (OtherComp :type "PrimitiveComponent Object Reference") (OtherBodyIndex :type Integer) (bFromSweep :type Boolean) (SweepResult :type "HitResult Structure (by ref)"))
  ;[0.2384 1 0.3654] E UI
  (cast `/Game/FP_Horror_Starter_Kit/PlayerCharacterExample/Blueprints/FirstPersonCharacter` OtherActor)
  (`SceneComponent.SetVisibility` (`self.Billboard`) true false)
  (if (`self.InInspectMode`)
    (`SceneComponent.SetVisibility` (`self.Billboard`) false false)))

(event `InputAxisKey|MouseY`
  (params (AxisValue :type "Float (single-precision)"))
  ;[1 0.7242 0.3207] Inspect Rotation
  (if (`self.Rotating`)
    (`self.K2_SetActorRotation` (`KismetMathLibrary.ComposeRotators` (`self.K2_GetActorRotation`) (`KismetMathLibrary.MakeRotator` 0.0 (* AxisValue -5.0))))))

(event `self.Box.OnComponentEndOverlap`
  (params (OverlappedComponent :type "PrimitiveComponent Object Reference") (OtherActor :type "Actor Object Reference") (OtherComp :type "PrimitiveComponent Object Reference") (OtherBodyIndex :type Integer))
  ;[0.2384 1 0.3654] E UI
  (cast `/Game/FP_Horror_Starter_Kit/PlayerCharacterExample/Blueprints/FirstPersonCharacter` OtherActor)
  (`SceneComponent.SetVisibility` (`self.Billboard`) false false))

(event `self.ReceiveBeginPlay`
  ;[0.2384 1 0.3654] E UI
  (`SceneComponent.SetVisibility` (`self.Billboard`) false false))

(event `Key|MouseScrollUp`
  (params (Key :type "Key Structure"))
  (bind _returnvalue (`GameplayStatics.GetPlayerCameraManager` 0))
  ;[0.5372 1 0.376] Inspect Zoom
  (:`Pressed`
    (bind _output_get (set `self.ZoomLevel` (`KismetMathLibrary.Clamp` (+ (`self.ZoomLevel`) 1) 1 20)))
    (if (< _output_get 20)
      (`self.K2_SetActorLocation` (+ (`PlayerCameraManager.GetCameraLocation` _returnvalue) (* (`KismetMathLibrary.GetForwardVector` (`PlayerCameraManager.GetCameraRotation` _returnvalue)) (* (`self.ZoomLevel`) 20.0)))))))

(event `Key|MouseScrollDown`
  (params (Key :type "Key Structure"))
  (bind _returnvalue (`GameplayStatics.GetPlayerCameraManager` 0))
  ;[0.5372 1 0.376] Inspect Zoom
  (:`Pressed`
    (bind _output_get (set `self.ZoomLevel` (`KismetMathLibrary.Clamp` (- (`self.ZoomLevel`) 1) 1 20)))
    (if (> _output_get 1)
      (`self.K2_SetActorLocation` (+ (`PlayerCameraManager.GetCameraLocation` _returnvalue) (* (`KismetMathLibrary.GetForwardVector` (`PlayerCameraManager.GetCameraRotation` _returnvalue)) (* (`self.ZoomLevel`) 20.0)))))))

(fn `DropItem`
  (bind _returnvalue (`GameplayStatics.GetPlayerCameraManager` 0))
  (bind _mesh (`self.Mesh`))
  (`Widget.SetVisibility` (`self.Inspection Controls`) "Hidden")
  (`self.K2_DetachFromActor` "KeepWorld" "KeepWorld" "KeepWorld")
  (`self.K2_SetActorLocation` (+ (`PlayerCameraManager.GetCameraLocation` _returnvalue) (* (`KismetMathLibrary.GetForwardVector` (`PlayerCameraManager.GetCameraRotation` _returnvalue)) 200.0)))
  (`PrimitiveComponent.SetSimulatePhysics` _mesh true)
  (`PrimitiveComponent.SetCollisionEnabled` _mesh "QueryAndPhysics")
  (set `self.InInspectMode` false)
  (`/Engine/EditorBlueprintResources/StandardMacros.DoOnce` false
    (:`Completed`
      (`GameplayStatics.PlaySoundAtLocation` "/Engine/VREditor/Sounds/UI/Object_PickUp.Object_PickUp" (0.0 0.0 0.0) (struct) 1.0 1.0 0.0 null null null))))

(fn `Pick Up`
  (bind _mesh (`self.Mesh`))
  (bind _returnvalue (`|CreateWidget` "/Game/Ben/Blueprints/InspectionUI/UI_Inspection_Controls.UI_Inspection_Controls_C"))
  (bind _output_get (set `self.Inspection Controls` _returnvalue))
  (`Widget.SetVisibility` _output_get "Visible")
  (`UserWidget.AddToViewport` _output_get 0)
  (`SceneComponent.SetVisibility` (`self.Billboard`) true false)
  (`self.K2_AttachToComponent` self (`/Game/FP_Horror_Starter_Kit/PlayerCharacterExample/Blueprints/FirstPersonCharacter.ItemHold` (`self.Player Character`)) "None" "SnapToTarget" "SnapToTarget" "KeepRelative" true)
  (`PrimitiveComponent.SetSimulatePhysics` _mesh false)
  (`PrimitiveComponent.SetCollisionEnabled` _mesh "NoCollision")
  (set `/Game/FP_Horror_Starter_Kit/PlayerCharacterExample/Blueprints/FirstPersonCharacter.CurrentHeld` self (`self.Player Character`))
  (set `self.InInspectMode` true)
  (`/Engine/EditorBlueprintResources/StandardMacros.DoOnce` false
    (:`Completed`
      (`GameplayStatics.PlaySoundAtLocation` "/Game/Ben/AtompshericSounds/SM_PickUp.SM_PickUp" (0.0 0.0 0.0) (struct) 1.0 1.0 0.0 null null null))))

(fn `StartInspect`
  (bind _returnvalue (`GameplayStatics.GetPlayerController` 0))
  (bind _returnvalue_2 (`GameplayStatics.GetPlayerCameraManager` 0))
  (`SceneComponent.SetVisibility` (`self.Billboard`) false false)
  (`Widget.SetVisibility` (`self.Inspection Controls`) "Hidden")
  (bind _returnvalue_3 (`|CreateWidget` "/Game/Ben/Blueprints/InspectionUI/UI_InspectionScreen.UI_InspectionScreen_C" null (`self.ItemDescription`)))
  (bind _output_get (set `self.InspectionUI` _returnvalue_3))
  (`Widget.SetVisibility` _output_get "Visible")
  (`UserWidget.AddToViewport` _output_get 0)
  (`self.DisableInput` (`self.Player Character`) _returnvalue)
  (`self.EnableInput` _returnvalue)
  (`self.K2_SetActorLocation` (+ (`PlayerCameraManager.GetCameraLocation` _returnvalue_2) (* (`KismetMathLibrary.GetForwardVector` (`PlayerCameraManager.GetCameraRotation` _returnvalue_2)) 200.0))))

(fn `Stop Inspect`
  (bind _returnvalue (`GameplayStatics.GetPlayerController` 0))
  (`Widget.SetVisibility` (`self.Inspection Controls`) "Visible")
  (`Widget.SetVisibility` (`self.InspectionUI`) "Hidden")
  (`self.DisableInput` _returnvalue)
  (`self.EnableInput` (`self.Player Character`) _returnvalue)
  (`self.K2_SetActorRelativeLocation` (0.0 0.0 0.0))
  (`self.K2_SetActorRelativeRotation` (struct)))

(fn `UserConstructionScript`)