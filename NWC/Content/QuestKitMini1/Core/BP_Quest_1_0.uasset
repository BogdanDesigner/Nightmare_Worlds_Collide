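; Button-sequence puzzle actor that requires two randomly shuffled codes to be entered in a row before firing OnWin.
; Construction script builds a row of textured, clickable buttons with lights, tagging each button with its index.
; BeginPlay generates both codes and passes them to the BP_Quest_1_1 with matching ID.
; Correct clicks light buttons; completing the first code lights a win lamp and switches codes, while any mistake clears progress.
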(event `self.ReceiveBeginPlay`
  (`self.CodeGeneration`)
  (set `self.Code_1` (`self.Code`))
  (`self.CodeGeneration`)
  (set `self.Code_2` (`self.Code`))
  (set `self.Code` (`self.Code_1`))
  (bind _outactors (`GameplayStatics.GetAllActorsOfClass` "/Game/QuestKitMini1/Core/BP_Quest_1_1.BP_Quest_1_1_C"))
  (for _array_element _outactors
    (if (== (`self.ID`) (`/Game/QuestKitMini1/Core/BP_Quest_1_1.ID` _array_element))
      (`/Game/QuestKitMini1/Core/BP_Quest_1_1.GenerateCode` _array_element (`self.Code_1`) (`self.Code_2`))
      (set `self.Ok` true)
      (break)))
  (if (not (`self.Ok`))
    (`KismetSystemLibrary.PrintString` "Please, add \"BP_Quest2_1\" to world and set ID" true true (struct :`R` 1.0 :`B` 0.025346 :`A` 1.0))))

(fn `ButtonClick`
  (params (TouchedComponent :type "PrimitiveComponent Object Reference") (ButtonPressed :type "Key Structure" :default "None"))
  (bind _returnvalue (`KismetStringLibrary.Conv_StringToInt` (`KismetStringLibrary.Conv_NameToString` (`|GetArrayItem` (`ActorComponent.ComponentTags` TouchedComponent)))))
  (if (== (`|GetArrayItem` (`self.Code`) (`self.ClickIndex`)) _returnvalue)
    (`self.LightSwitch` _returnvalue)
    (`/Engine/EditorBlueprintResources/StandardMacros.IncrementInt` (`self.ClickIndex`)
      (:`  `
        (`self.CheckWin`)))
    (else
      (`self.OffAll`)
      (set `self.ClickIndex` 0)
      (`self.ResetWin`))))

(fn `CheckWin`
  (locals (isWin :type Boolean))
  (set `local.isWin` true)
  (for _array_element (`self.LightsStatus`)
    (if (not _array_element)
      (set `local.isWin` false)))
  (if (`local.isWin`)
    (bind _result (`/Engine/EditorBlueprintResources/StandardMacros.IncrementInt` (`self.Win`))
      (:`  `
        (if (== _result 2)
          (`self.onWin` self)
          (`PrimitiveComponent.SetMaterial` (`self.LightWin2`) 0 (`self.MaterialWin`))
          (else
            (`PrimitiveComponent.SetMaterial` (`self.LightWin1`) 0 (`self.MaterialWin`))
            (`self.OffAll`)
            (set `self.Code` (`self.Code_2`))))))))

(fn `CodeGeneration`
  (locals (Digital :type "Array of Integer") (RandomIndex :type Integer))
  (bind _digital (`local.Digital`))
  (`KismetArrayLibrary.Array_Clear` (`self.Code`))
  (for _index (range (+ (`self.CodeLen`) 1))
    (`KismetArrayLibrary.Array_Add` (`local.Digital`) _index))
  (for _ (range (+ (`self.CodeLen`) 1))
    (bind _output_get (set `local.RandomIndex` (`KismetMathLibrary.RandomInteger` (`KismetArrayLibrary.Array_Length` _digital))))
    (`KismetArrayLibrary.Array_Add` (`self.Code`) (`|GetArrayItem` _digital _output_get))
    (`KismetArrayLibrary.Array_Remove` _digital _output_get))
  (`self.DisplayCode`))

(fn `DisplayCode`
  (set `self.CodeStr` "")
  (for _array_element (`self.Code`)
    (set `self.CodeStr` (`KismetStringLibrary.Concat_StrStr` (`self.CodeStr`) (`KismetStringLibrary.Conv_IntToString` _array_element) " "))))

(fn `LightSwitch`
  (params (id :type Integer))
  (locals (NewStatus :type Boolean))
  (bind _lightsstatus (`self.LightsStatus`))
  (bind _output_get (set `local.NewStatus` (not (`|GetArrayItem` _lightsstatus id))))
  (`KismetArrayLibrary.Array_Set` _lightsstatus id _output_get)
  (`PrimitiveComponent.SetMaterial` (`|GetArrayItem` (`self.Lights`) id) 0 (select `bool` (`local.NewStatus`) :`false` (`self.MaterialOff`) :`true` (`self.MaterialOn`))))

(fn `OffAll`
  (bind _lightsstatus (`self.LightsStatus`))
  (for (_ _array_index) _lightsstatus
    (`KismetArrayLibrary.Array_Set` _lightsstatus _array_index)
    (`PrimitiveComponent.SetMaterial` (`|GetArrayItem` (`self.Lights`) _array_index) 0 (`self.MaterialOff`))
    (set `self.ClickIndex` 0)))

(fn `ResetWin`
  (set `self.Win` 0)
  (`PrimitiveComponent.SetMaterial` (`self.LightWin1`) 0 (`self.MaterialOff`)))

(fn `UserConstructionScript`
  (bind (_startposition_x _startposition_y _startposition_z) (`KismetMathLibrary.BreakVector` (`self.StartPosition`)))
  (for _index (range (+ (`self.CodeLen`) 1))
    (bind _returnvalue (+ _startposition_y (`KismetMathLibrary.Conv_IntToDouble` (* _index -8))))
    (bind _returnvalue_2 (`AddComponent|NODE_AddStaticMeshComponent-0` :`RelativeTransform` (`KismetMathLibrary.MakeTransform` (`KismetMathLibrary.MakeVector` (+ _startposition_x -2.0) _returnvalue _startposition_z) (struct :`Roll` 180.0))))
    (`SceneComponent.K2_AttachToComponent` _returnvalue_2 (`self.DefaultSceneRoot`) "None" "KeepRelative" "KeepRelative" "KeepRelative" true)
    (bind _returnvalue_3 (`KismetMaterialLibrary.CreateDynamicMaterialInstance` "/Game/QuestKitMini1/Materials/M_Button1_Mat.M_Button1_Mat"))
    (`MaterialInstanceDynamic.SetTextureParameterValue` _returnvalue_3 "Texture" (`|GetArrayItem` (`self.T_Buttons`) _index))
    (`PrimitiveComponent.SetMaterial` _returnvalue_2 1 _returnvalue_3)
    (set `ActorComponent.ComponentTags` (`|MakeArray` (`KismetStringLibrary.Conv_StringToName` (`KismetStringLibrary.Conv_IntToString` _index))) _returnvalue_2)
    (add `PrimitiveComponent.OnClicked` _returnvalue_2 (`|CreateDelegate` :!event `ButtonClick`))
    (bind _returnvalue_4 (`AddComponent|NODE_AddStaticMeshComponent-2` :`RelativeTransform` (`KismetMathLibrary.MakeTransform` (`KismetMathLibrary.MakeVector` _startposition_x _returnvalue (+ _startposition_z 10.0)))))
    (`SceneComponent.K2_AttachToComponent` _returnvalue_4 (`self.DefaultSceneRoot`) "None" "KeepRelative" "KeepRelative" "KeepRelative" true)
    (`KismetArrayLibrary.Array_Add` (`self.Lights`) _returnvalue_4)
    (`KismetArrayLibrary.Array_Add` (`self.LightsStatus`))))