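; Wire-matching quest puzzle where the player links same-colored pins with cables; six connections turn the sphere green and fire the win call.
; Generation scatters randomly placed pins over two panels, shuffles colors between them and stores each color index as a component tag.
; Clicking a pin spawns a cable whose end follows a mouse trace; a matching click attaches it, otherwise it is destroyed.
; PlayerView changes cancel any unfinished cable.
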(event `self.ReceiveBeginPlay`
  (`self.Generation`)
  (add `PrimitiveComponent.OnClicked` (`self.Pins`) (`|CreateDelegate` :!event `PinClick`)))

(event `self.ReceiveTick`
  (params (DeltaSeconds :type "Float (single-precision)"))
  (bind _newcable (`self.NewCable`))
  (if (`self.isNewCable`)
    (if (`self.isInteractive`)
      (bind _returnvalue (`WidgetLayoutLibrary.GetMousePositionOnViewport`))
      (bind (_worldposition _worlddirection) (`GameplayStatics.DeprojectScreenToWorld` (`GameplayStatics.GetPlayerController` 0) (* _returnvalue (`WidgetLayoutLibrary.GetViewportScale`))))
      (bind _outhit (`KismetSystemLibrary.LineTraceSingle` :`Start` _worldposition :`End` (+ _worldposition (* _worlddirection (`self.Range`))) :`TraceChannel` "TraceTypeQuery1" :`DrawDebugType` "ForOneFrame" :`bIgnoreSelf` false))
      (`/Engine/EditorBlueprintResources/StandardMacros.IsValid` _newcable
        (:`Is Valid`
          (set `CableComponent.EndLocation` (`KismetMathLibrary.InverseTransformLocation` (`self.GetTransform`) (select `bool` (`GameplayStatics.BreakHitResult` _outhit) :`false` (`.TraceEnd` (`GameplayStatics.BreakHitResult` _outhit)) :`true` (`.Location` (`GameplayStatics.BreakHitResult` _outhit)))) _newcable))))))

(fn `Generation`
  (locals (ColorsTmp :type "Array of LinearColor Structure") (RandomIndex :type Integer) (PanelNum :type Byte))
  (bind _pins (`self.Pins`))
  (bind _left_points (`self.Left_Points`))
  (bind _colorstmp (`local.ColorsTmp`))
  (bind (_returnvalue_x _returnvalue_y _returnvalue_z) (`KismetMathLibrary.BreakVector` (select `byte` (`local.PanelNum`) :`0` (`self.StartPositionL`) :`1` (`self.StartPositionR`))))
  (for _array_element _pins
    (`ActorComponent.K2_DestroyComponent` _array_element))
  (`KismetArrayLibrary.Array_Clear` _pins)
  (for _index (range 2)
    (set `local.PanelNum` (`KismetMathLibrary.Conv_IntToByte` _index))
    (`KismetArrayLibrary.Array_Clear` (`self.Left_Points`))
    (for _index_2 (range 6)
      (for _index_3 (range 6)
        (`KismetArrayLibrary.Array_Add` (`self.Left_Points`) (`KismetMathLibrary.MakeVector` (+ _returnvalue_x -2.0) (+ _returnvalue_y (`KismetMathLibrary.Conv_IntToDouble` (* _index_2 -8))) (+ _returnvalue_z (`KismetMathLibrary.Conv_IntToDouble` (* _index_3 -8)))))))
    (for _ (range 30)
      (`KismetArrayLibrary.Array_Remove` _left_points (`KismetMathLibrary.RandomInteger` (- (`KismetArrayLibrary.Array_Length` _left_points) 1))))
    (set `local.ColorsTmp` (`self.Colors`))
    (for _array_element_2 (`self.Left_Points`)
      (bind _returnvalue (`AddComponent|NODE_AddStaticMeshComponent-0` :`RelativeTransform` (`KismetMathLibrary.MakeTransform` _array_element_2 (struct :`Pitch` 90.0))))
      (`KismetArrayLibrary.Array_Add` (`self.Pins`) _returnvalue)
      (`SceneComponent.K2_AttachToComponent` _returnvalue (select `byte` (`local.PanelNum`) :`0` (`self.CubeR`) :`1` (`self.CubeL`) :!type "SceneComponent Object Reference") "None" "KeepRelative" "KeepRelative" "KeepRelative" true)
      (bind _returnvalue_2 (`KismetMaterialLibrary.CreateDynamicMaterialInstance` "/Game/QuestKitMini1/Materials/MI_BasePin.MI_BasePin"))
      (bind _output_get (set `local.RandomIndex` (`KismetMathLibrary.RandomInteger` (- (`KismetArrayLibrary.Array_Length` _colorstmp) 1))))
      (bind _output (`|GetArrayItem` _colorstmp _output_get))
      (set `ActorComponent.ComponentTags` (`|MakeArray` (`KismetStringLibrary.Conv_StringToName` (`KismetStringLibrary.Conv_IntToString` (`KismetArrayLibrary.Array_Find` (`self.Colors`) _output)))) _returnvalue)
      (`MaterialInstanceDynamic.SetVectorParameterValue` _returnvalue_2 "Color" _output)
      (`PrimitiveComponent.SetMaterial` _returnvalue 0 _returnvalue_2)
      (`KismetArrayLibrary.Array_Remove` (`local.ColorsTmp`) (`local.RandomIndex`)))))

(fn `PinClick`
  (params (TouchedComponent :type "PrimitiveComponent Object Reference") (ButtonPressed :type "Key Structure" :default "None"))
  (bind _newcable (`self.NewCable`))
  (bind _currentpin (`self.CurrentPin`))
  (bind _output (`|GetArrayItem` (`ActorComponent.ComponentTags` TouchedComponent)))
  (if (`self.isNewCable`)
    (if (and (== _output (`|GetArrayItem` (`ActorComponent.ComponentTags` _currentpin))) (not (== TouchedComponent _currentpin)))
      ;[1 1 1] Valid, connect
      (set `CableComponent.EndLocation` (0.0 0.0 2.0) _newcable)
      (`MaterialInstanceDynamic.SetVectorParameterValue` (cast `MaterialInstanceDynamic` (`PrimitiveComponent.GetMaterial` _newcable 0) :!pure true) "Color" (`|GetArrayItem` (`self.Colors`) (`KismetStringLibrary.Conv_StringToInt` (`KismetStringLibrary.Conv_NameToString` _output))))
      (`CableComponent.SetAttachEndToComponent` _newcable TouchedComponent "None")
      (set `self.isNewCable` false)
      (set `self.CurrentPin` null)
      (bind _result (`/Engine/EditorBlueprintResources/StandardMacros.IncrementInt` (`self.TotalCabels`))
        (:`  `
          (if (== _result 6)
            (`self.Win`))))
      (else
        ;[1 1 1] No valid!
        (`ActorComponent.K2_DestroyComponent` (`self.NewCable`))
        (set `self.isNewCable` false)))
    (else
      ;[1 1 1] Add new cable
      (set `self.CurrentPin` TouchedComponent)
      (bind _returnvalue (`AddComponent|NODE_AddCableComponent-0` :`RelativeTransform` (`KismetMathLibrary.MakeTransform` (0.0 0.0 2.0))))
      (bind _output_get (set `self.NewCable` _returnvalue))
      (`SceneComponent.K2_AttachToComponent` _returnvalue TouchedComponent "None" "KeepRelative" "KeepRelative" "KeepRelative" true)
      (bind _returnvalue_2 (`KismetMaterialLibrary.CreateDynamicMaterialInstance` "/Game/QuestKitMini1/Materials/MI_Cable.MI_Cable"))
      (`PrimitiveComponent.SetMaterial` _output_get 0 _returnvalue_2)
      (set `self.isNewCable` true))))

(fn `PlayerView`
  (params (isIn :type Boolean))
  (`parent.PlayerView` isIn)
  (if (`self.isNewCable`)
    (set `self.isNewCable` false)
    (`ActorComponent.K2_DestroyComponent` (`self.NewCable`))
    (set `self.isNewCable` false)))

(fn `UserConstructionScript`
  (locals (ColorsTmp :type "Array of LinearColor Structure") (RandomIndex :type Integer) (PanelNum :type Byte)))

(fn `Win`
  (`PrimitiveComponent.SetMaterial` (`self.Sphere`) 0 "/Game/QuestKitMini1/Materials/MI_GreenEmissive.MI_GreenEmissive")
  (`self.onWin` self))