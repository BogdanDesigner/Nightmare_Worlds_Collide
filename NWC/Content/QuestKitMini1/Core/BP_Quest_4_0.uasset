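; BP_Quest_4_0 is a Simon-style memory puzzle on nine buttons that notifies on win once a random five-step sequence is repeated.
; When the player enters view, timers blink a growing prefix of the sequence while input is locked.
; Correct presses flash green and advance rounds and progress meshes; a wrong press flashes red and restarts with a new sequence.
; Material swaps drive button and progress feedback, with text showing the current phase.
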(event `self.ReceiveBeginPlay`
  ;[1 1 1] Bind all buttons onClick
  (for _array_element (`self.Buttons`)
    (add `PrimitiveComponent.OnClicked` _array_element (delegate `onClick`))))

(event `onClick`
  (params (TouchedComponent :type "PrimitiveComponent Object Reference") (ButtonPressed :type "Key Structure" :default "None"))
  ;[1 1 1] Bind all buttons onClick
  (`self.ButtonClick` (- (`KismetStringLibrary.Conv_StringToInt` (`KismetSystemLibrary.GetObjectName` TouchedComponent)) 1)))

(event `ButtonClick`
  (params (Int :type Integer))
  (if (`self.EnableImput`)
    (set `self.EnableImput` false)
    ;[1 1 1] Check valid
    (if (== Int (`|GetArrayItem` (`self.Password`) (`self.InputIndex`)))
      ;[1 1 1] Valid
      (`self.SetButtonStyle` Int 1)
      (bind _returnvalue (`KismetSystemLibrary.K2_SetTimerDelegate` (delegate `ResumeButtonStyleOk`) (`self.BlinkDelay`)))
      (set `self.ShowButtonTimer` _returnvalue)
      (else
        ;[1 1 1] Not valid
        (`self.SetButtonStyle` Int 2)
        (bind _returnvalue_2 (`KismetSystemLibrary.K2_SetTimerDelegate` (delegate `ResumeStyleButtonErr`) (`self.BlinkDelay`)))
        (set `self.ShowButtonTimer` _returnvalue_2)))))

(event `ResumeButtonStyleOk`
  (`self.SetButtonStyle` (stale `ButtonClick` Int))
  ;[1 1 1] Check code and Win
  (bind _result (`/Engine/EditorBlueprintResources/StandardMacros.IncrementInt` (`self.InputIndex`))
    (:`  `
      (if (== _result (`self.NeedInputIndex`))
        (bind _result_2 (`/Engine/EditorBlueprintResources/StandardMacros.IncrementInt` (`self.NeedInputIndex`))
          (:`  `
            (set `self.InputIndex` 0)
            (`self.UpdateProgress`)
            (if (== _result_2 (+ (`KismetArrayLibrary.Array_Length` (`self.Password`)) 1))
              (`self.SetInfo` 2)
              (`self.onWin` self)
              (else
                (set `self.EnableImput` true)
                (`self.ShowPass` _result_2)))))
        (else
          (set `self.EnableImput` true))))))

(event `ResumeStyleButtonErr`
  (`self.SetButtonStyle` (stale `ButtonClick` Int))
  (`self.Reset`)
  (`self.ShowPass` 1))

(event `ShowPass`
  (params (ShowIndexMax :type Integer))
  ;[1 1 1] Show code
  (`self.SetInfo` 0)
  (set `self.ShowIndexMax` ShowIndexMax)
  (set `self.ShowIndex` 0)
  (set `self.EnableImput` false)
  (bind _returnvalue (`KismetSystemLibrary.K2_SetTimerDelegate` (delegate `onShowTick`) 1.0 true))
  (set `self.ShowTimer` _returnvalue))

(event `onShowTick`
  ;[1 1 1] Show code
  (`self.SetButtonStyle` (`|GetArrayItem` (`self.Password`) (`self.ShowIndex`)) 1)
  (`KismetSystemLibrary.Delay` (`self.BlinkDelay`))
  (bind _returnvalue (`KismetSystemLibrary.K2_SetTimerDelegate` (delegate `ResumeStyleButton`) (`self.BlinkDelay`)))
  (set `self.ShowButtonTimer` _returnvalue))

(event `ResumeStyleButton`
  ;[1 1 1] Show code
  (`self.SetButtonStyle` (`|GetArrayItem` (`self.Password`) (`self.ShowIndex`)))
  (bind _result (`/Engine/EditorBlueprintResources/StandardMacros.IncrementInt` (`self.ShowIndex`))
    (:`  `
      (if (== _result (`self.ShowIndexMax`))
        (set `self.EnableImput` true)
        (`KismetSystemLibrary.K2_ClearAndInvalidateTimerHandle` (`self.ShowTimer`))
        (`self.SetInfo` 1)))))

(fn `GeneratePass`
  (locals (Values :type "Array of Integer"))
  (`KismetArrayLibrary.Array_Clear` (`self.Password`))
  (for _index (range 9)
    (`KismetArrayLibrary.Array_Add` (`local.Values`) _index))
  (for _ (range 5)
    (`KismetArrayLibrary.Array_Add` (`self.Password`) (`KismetArrayLibrary.Array_Random` (`local.Values`)))))

(fn `PlayerView`
  (params (isIn :type Boolean))
  (`parent.PlayerView` isIn)
  (if isIn
    (`self.Reset`)
    (`self.ShowPass` 1)
    (else
      (`self.Reset`)
      (`self.SetInfo` 3))))

(fn `Reset`
  (`KismetSystemLibrary.K2_ClearAndInvalidateTimerHandle` (`self.ShowButtonTimer`))
  (`KismetSystemLibrary.K2_ClearAndInvalidateTimerHandle` (`self.ShowTimer`))
  (`self.GeneratePass`)
  (set `self.InputIndex` 0)
  (set `self.NeedInputIndex` 1)
  (`self.UpdateProgress`)
  (for (_ _array_index) (`self.Buttons`)
    (`self.SetButtonStyle` _array_index)))

(fn `SetButtonStyle`
  (params (Index :type Integer) (Style :type Byte))
  (bind _returnvalue (select `byte` Style :`0` "/Game/QuestKitMini1/Materials/MI_BaseC.MI_BaseC" :`1` "/Game/QuestKitMini1/Materials/MI_GreenEmissive.MI_GreenEmissive" :`2` "/Game/QuestKitMini1/Materials/MI_RedEmissive.MI_RedEmissive" :!type "MaterialInterface Object Reference"))
  (bind _output (`|GetArrayItem` (`self.Buttons`) Index))
  (`PrimitiveComponent.SetMaterial` _output 0 _returnvalue)
  (`PrimitiveComponent.SetMaterial` _output 1 _returnvalue))

(fn `SetInfo`
  (params (Index :type Byte))
  (`TextRenderComponent.K2_SetText` (`self.TextRenderAction`) (select `byte` Index :`0` (`self.InfoSee`) :`1` (`self.InfoInput`) :`2` (`self.InfoWin`) :`3` (`self.InfoWait`))))

(fn `UpdateProgress`
  (for (_array_element _array_index) (`self.ProgressSM`)
    (`PrimitiveComponent.SetMaterial` _array_element 0 (select `bool` (> _array_index (- (`self.NeedInputIndex`) 2)) :`false` "/Game/QuestKitMini1/Materials/MI_GreenEmissive.MI_GreenEmissive" :`true` "/Game/QuestKitMini1/Materials/MI_BaseB.MI_BaseB" :!type "MaterialInterface Object Reference"))))

(fn `UserConstructionScript`
  (set `self.Buttons` (`|MakeArray` (`self.1`) (`self.2`) (`self.3`) (`self.4`) (`self.5`) (`self.6`) (`self.7`) (`self.8`) (`self.9`)))
  (set `self.ProgressSM` (`|MakeArray` (`self.StaticMesh4`) (`self.StaticMesh3`) (`self.StaticMesh2`) (`self.StaticMesh1`) (`self.StaticMesh`))))